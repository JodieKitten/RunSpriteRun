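; Character Blueprint that sets up a layered parallax background and animates a floating heart sprite.
; On BeginPlay, each sprite child of StaticBackground gets a dynamic material instance, stored in DynamicLayers, with its ParallaxMultiplier parameter set from the index-matched ParallaxMultipliers array.
; While HeartSprite is visible, Tick accumulates time in Amplitude and applies a sine-based local Z offset to bob it.
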(event `self.ReceiveBeginPlay`
  (for (_array_element _array_index) (`SceneComponent.GetChildrenComponents` (`self.StaticBackground`) false)
    (bind _aspaper_sprite_component (cast `PaperSpriteComponent` _array_element))
    (bind _returnvalue (`PrimitiveComponent.CreateDynamicMaterialInstance` _aspaper_sprite_component 0 null "None"))
    (`KismetArrayLibrary.Array_Add` (`self.DynamicLayers`) _returnvalue)
    (`MaterialInstanceDynamic.SetScalarParameterValue` _returnvalue "ParallaxMultiplier" (`|GetArrayItem` (`self.ParallaxMultipliers`) _array_index))))

(event `self.ReceiveTick`
  (params (DeltaSeconds :type "Float (single-precision)"))
  (bind _amplitude (`self.Amplitude`))
  (bind _heartsprite (`self.HeartSprite`))
  (if (`SceneComponent.IsVisible` _heartsprite)
    (set `self.Amplitude` (+ DeltaSeconds _amplitude))
    (`SceneComponent.K2_AddLocalOffset` _heartsprite (`KismetMathLibrary.MakeVector` 0.0 0.0 (* 0.1 (`KismetMathLibrary.Sin` (* _amplitude 5.0)))) false false)))

(fn `UserConstructionScript`)