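; BP_FishReward is a fish reward actor that bobs gently up and down in the world.
; Tick accumulates elapsed time and uses its sine to apply a small vertical world offset each frame, so the motion depends on frame rate.
; The Box end-overlap event is empty, and disconnected logic that would cast to BP_Character and make the box block Pawns never runs.
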(event `self.ReceiveTick`
  (params (DeltaSeconds :type "Float (single-precision)"))
  (bind _newvar (`self.NewVar`))
  (set `self.NewVar` (+ DeltaSeconds _newvar))
  (`self.K2_AddActorWorldOffset` (`KismetMathLibrary.MakeVector` 0.0 0.0 (* 0.1 (`KismetMathLibrary.Sin` (* _newvar 5.0))))))

(event `self.Box.OnComponentEndOverlap`
  (params (OverlappedComponent :type "PrimitiveComponent Object Reference") (OtherActor :type "Actor Object Reference") (OtherComp :type "PrimitiveComponent Object Reference") (OtherBodyIndex :type Integer)))

(fn `UserConstructionScript`)